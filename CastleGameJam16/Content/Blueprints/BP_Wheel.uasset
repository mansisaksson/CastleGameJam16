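; BP_Wheel is a damageable, repairable wheel for BP_Cart, found at BeginPlay.
; Each tick it spins with cart speed, drives a dynamic material scalar from health, and scales broken-sound volume by speed.
; Overlapping a BP_BreakBox destroys the box and deals full damage if its break flag matches the wheel's side.
; Zero health shows particles, plays sound and applies the cart's break force; full repair reverses all three.
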(event `self.ReceiveBeginPlay`
  (bind _outactors (`GameplayStatics.GetAllActorsOfClass` "/Game/Blueprints/BP_Cart.BP_Cart_C"))
  (for _array_element _outactors
    (set `self.Cart` _array_element)
    (`SceneComponent.SetVisibility` (`self.ParticleSystem`) false false)
    (bind _returnvalue (`KismetMaterialLibrary.CreateDynamicMaterialInstance` "/Game/Assets/Train/Wheel_Metal.Wheel_Metal"))
    (bind _output_get (set `self.MatInst` _returnvalue))
    (`PrimitiveComponent.SetMaterial` (`self.Wheel`) 1 _output_get)))

(event `self.ReceiveTick`
  (params (DeltaSeconds :type "Float (single-precision)"))
  (bind _cart (`self.Cart`))
  (`|ExecutionSequence`
    (:`then_0`
      ;[1 1 1] Rotate Wheels + Change Wheel Color
      (`SceneComponent.K2_AddLocalRotation` (`self.Wheel`) (`KismetMathLibrary.MakeRotator` (/ (`/Game/Blueprints/BP_Cart.CurrentSpeed` (`self.Cart`)) (`self.SpinSpeed`))) false false)
      (`MaterialInstanceDynamic.SetScalarParameterValue` (`self.MatInst`) "Scalar" (/ (`self.Health`) 100.0)))
    (:`then_1`
      ;[1 1 1] Sound Bound to speed
      (`AudioComponent.SetVolumeMultiplier` (`self.BrokenSound`) (/ (`/Game/Blueprints/BP_Cart.CurrentSpeed` _cart) (`/Game/Blueprints/BP_Cart.MaxSpeed` _cart))))))

(event `self.Wheel.OnComponentBeginOverlap`
  (params (OverlappedComponent :type "PrimitiveComponent Object Reference") (OtherActor :type "Actor Object Reference") (OtherComp :type "PrimitiveComponent Object Reference") (OtherBodyIndex :type Integer) (bFromSweep :type Boolean) (SweepResult :type "HitResult Structure (by ref)"))
  (bind _asbp_break_box (cast `/Game/Blueprints/BP_BreakBox` OtherActor))
  (if (and (not (`self.IsRightWheel`)) (`/Game/Blueprints/BP_BreakBox.ForceLeftBreak` _asbp_break_box))
    (`self.ApplyDamage` 100.0))
  (if (and (`self.IsRightWheel`) (`/Game/Blueprints/BP_BreakBox.ForceRightBreak` _asbp_break_box))
    (`self.ApplyDamage` 100.0))
  (`self.K2_DestroyActor` _asbp_break_box))

(fn `ApplyDamage`
  (params (Damage :type "Float (double-precision)"))
  (bind _output_get (set `self.Health` (`KismetMathLibrary.FClamp` (- (`self.Health`) Damage) 0.0 100.0)))
  (if (<= _output_get 0.0)
    (`SceneComponent.SetVisibility` (`self.ParticleSystem`) true false)
    (if (not (`self.IsBroken`))
      (`/Game/Blueprints/BP_Cart.ApplyBreakForce` (`self.Cart`))
      (`AudioComponent.Play` (`self.BrokenSound`) 0.0))
    (set `self.IsBroken` true)))

(fn `Repair`
  (params (Amount :type "Float (double-precision)"))
  (bind _output_get (set `self.Health` (`KismetMathLibrary.FClamp` (+ Amount (`self.Health`)) 0.0 100.0)))
  (if (>= _output_get 100.0)
    (`SceneComponent.SetVisibility` (`self.ParticleSystem`) false false)
    (if (`self.IsBroken`)
      (`/Game/Blueprints/BP_Cart.RemoveBreakForce` (`self.Cart`))
      (`AudioComponent.Stop` (`self.BrokenSound`)))
    (set `self.IsBroken` false)))

(fn `UserConstructionScript`)