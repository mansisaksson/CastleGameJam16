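; VR player Blueprint with floor-tracked HMD and two motion-controller hands that highlight, grab and release BP_Utility objects.
; Tick moves both hand points to the controller poses and stores a per-hand velocity value from position change multiplied by delta time.
; Hand overlaps set the highlighted utility, which a trigger press snaps to that hand's socket.
; Grabbing from the other hand transfers ownership, and trigger release calls the utility's Release.
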(event `self.ReceiveBeginPlay`
  (`HeadMountedDisplayFunctionLibrary.EnableHMD` true)
  (`HeadMountedDisplayFunctionLibrary.SetTrackingOrigin` "Floor")
  (set `self.OldLeftHandPosition` (`SteamVRFunctionLibrary.GetHandPositionAndOrientation` 0 "Left")))

(event `self.ReceiveTick`
  (params (DeltaSeconds :type "Float (single-precision)"))
  (bind _outposition (`SteamVRFunctionLibrary.GetHandPositionAndOrientation` 0 "Right"))
  (bind (_outposition_2 _outorientation) (`SteamVRFunctionLibrary.GetHandPositionAndOrientation` 0 "Right"))
  (bind _outposition_3 (`SteamVRFunctionLibrary.GetHandPositionAndOrientation` 0 "Left"))
  (bind (_outposition_4 _outorientation_2) (`SteamVRFunctionLibrary.GetHandPositionAndOrientation` 0 "Left"))
  (bind _lefthand_point (`self.LeftHand_Point`))
  (bind _righthand_point (`self.RightHand_Point`))
  (`|ExecutionSequence`
    (:`then_0`
      ;[1 1 1] Update Vive Controllers
      (`SceneComponent.K2_SetRelativeLocation` _lefthand_point _outposition_4 false false)
      (`SceneComponent.K2_SetRelativeRotation` _lefthand_point _outorientation_2 false false)
      (`SceneComponent.K2_SetRelativeLocation` _righthand_point _outposition_2 false false)
      (`SceneComponent.K2_SetRelativeRotation` _righthand_point _outorientation false false))
    (:`then_1`
      ;[1 1 1] Calculate Hand Velocity
      (set `self.RightHandVelocity` (* (`KismetMathLibrary.VSize` (- _outposition (`self.OldRightHandPosition`))) (`GameplayStatics.GetWorldDeltaSeconds`)))
      (set `self.OldRightHandPosition` _outposition)
      (set `self.LeftHandVelocity` (* (`KismetMathLibrary.VSize` (- _outposition_3 (`self.OldLeftHandPosition`))) (`GameplayStatics.GetWorldDeltaSeconds`)))
      (set `self.OldLeftHandPosition` _outposition_3))))

(event `self.Right Hand.OnComponentBeginOverlap`
  (params (OverlappedComponent :type "PrimitiveComponent Object Reference") (OtherActor :type "Actor Object Reference") (OtherComp :type "PrimitiveComponent Object Reference") (OtherBodyIndex :type Integer) (bFromSweep :type Boolean) (SweepResult :type "HitResult Structure (by ref)"))
  ;[1 1 1] Add Highlight
  (`/Engine/EditorBlueprintResources/StandardMacros.IsValid` (`self.RightUtility`)
    (:`Is Not Valid`
      (bind _asbp_utility (cast `/Game/Blueprints/BP_Utility` OtherActor))
      (bind _output_get (set `self.RightHighlightedUtility` _asbp_utility))
      (`/Game/Blueprints/BP_Utility.SetHighLight` _output_get true))))

(event `self.Left Hand.OnComponentBeginOverlap`
  (params (OverlappedComponent :type "PrimitiveComponent Object Reference") (OtherActor :type "Actor Object Reference") (OtherComp :type "PrimitiveComponent Object Reference") (OtherBodyIndex :type Integer) (bFromSweep :type Boolean) (SweepResult :type "HitResult Structure (by ref)"))
  ;[1 1 1] Add Highlight
  (`/Engine/EditorBlueprintResources/StandardMacros.IsValid` (`self.LeftUtility`)
    (:`Is Not Valid`
      (bind _asbp_utility (cast `/Game/Blueprints/BP_Utility` OtherActor))
      (bind _output_get (set `self.LeftHighlightedUtility` _asbp_utility))
      (`/Game/Blueprints/BP_Utility.SetHighLight` _output_get true))))

(event `self.Right Hand.OnComponentEndOverlap`
  (params (OverlappedComponent :type "PrimitiveComponent Object Reference") (OtherActor :type "Actor Object Reference") (OtherComp :type "PrimitiveComponent Object Reference") (OtherBodyIndex :type Integer))
  ;[1 1 1] Remove Highlight
  (bind _asbp_utility (cast `/Game/Blueprints/BP_Utility` OtherActor))
  (`/Game/Blueprints/BP_Utility.SetHighLight` _asbp_utility false)
  (if (== _asbp_utility (`self.RightHighlightedUtility`))
    (set `self.RightHighlightedUtility` null)))

(event `self.Left Hand.OnComponentEndOverlap`
  (params (OverlappedComponent :type "PrimitiveComponent Object Reference") (OtherActor :type "Actor Object Reference") (OtherComp :type "PrimitiveComponent Object Reference") (OtherBodyIndex :type Integer))
  ;[1 1 1] Remove Highlight
  (bind _asbp_utility (cast `/Game/Blueprints/BP_Utility` OtherActor))
  (`/Game/Blueprints/BP_Utility.SetHighLight` _asbp_utility false)
  (if (== _asbp_utility (`self.LeftHighlightedUtility`))
    (set `self.LeftHighlightedUtility` null)))

(event `Key|MotionController_Right_Trigger`
  (params (Key :type "Key Structure" :default "AnyKey"))
  (bind _righthighlightedutility (`self.RightHighlightedUtility`))
  (bind _rightutility (`self.RightUtility`))
  ;[1 1 1] PickUp Right Hand
  (:`Pressed`
    (`/Engine/EditorBlueprintResources/StandardMacros.IsValid` (`self.RightUtility`)
      (:`Is Not Valid`
        (`/Engine/EditorBlueprintResources/StandardMacros.IsValid` _righthighlightedutility
          (:`Is Valid`
            (if (== (`self.RightHighlightedUtility`) (`self.LeftUtility`))
              (set `self.LeftUtility` null))
            (bind _output_get (set `self.RightUtility` _righthighlightedutility))
            (`/Game/Blueprints/BP_Utility.SetHighLight` _output_get false)
            (`self.K2_AttachToComponent` (`self.RightHighlightedUtility`) (`self.Right Hand`) "Socket" "SnapToTarget" "SnapToTarget" "KeepWorld" true)
            (set `self.RightHighlightedUtility` null))))))
  (:`Released`
    (`/Engine/EditorBlueprintResources/StandardMacros.IsValid` _rightutility
      (:`Is Valid`
        (`/Game/Blueprints/BP_Utility.Release` _rightutility)
        (set `self.RightUtility` null)))))

(event `Key|MotionController_Left_Trigger`
  (params (Key :type "Key Structure" :default "AnyKey"))
  (bind _leftutility (`self.LeftUtility`))
  (bind _lefthighlightedutility (`self.LeftHighlightedUtility`))
  ;[1 1 1] PickUp Left Hand
  (:`Pressed`
    (`/Engine/EditorBlueprintResources/StandardMacros.IsValid` (`self.LeftUtility`)
      (:`Is Not Valid`
        (`/Engine/EditorBlueprintResources/StandardMacros.IsValid` _lefthighlightedutility
          (:`Is Valid`
            (if (== (`self.LeftHighlightedUtility`) (`self.RightUtility`))
              (set `self.RightUtility` null))
            (bind _output_get (set `self.LeftUtility` _lefthighlightedutility))
            (`/Game/Blueprints/BP_Utility.SetHighLight` _output_get false)
            (`self.K2_AttachToComponent` (`self.LeftHighlightedUtility`) (`self.Left Hand`) "Socket" "SnapToTarget" "SnapToTarget" "KeepWorld" true)
            (set `self.LeftHighlightedUtility` null))))))
  (:`Released`
    (`/Engine/EditorBlueprintResources/StandardMacros.IsValid` _leftutility
      (:`Is Valid`
        (`/Game/Blueprints/BP_Utility.Release` _leftutility)
        (set `self.LeftUtility` null)))))

(fn `UserConstructionScript`)