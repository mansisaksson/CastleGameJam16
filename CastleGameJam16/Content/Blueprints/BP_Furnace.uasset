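; BP_Furnace is a furnace actor whose health steadily degrades over time and can be restored through a Repair function.
; BeginPlay applies a dynamic glow material to the mesh and starts the engine sound.
; Tick drains clamped Health at DegradationSpeed, driving both the material's Glow parameter and the sound's volume from the health fraction.
; Repair adds clamped health and updates the glow immediately.
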(event `self.ReceiveBeginPlay`
  (bind _returnvalue (`KismetMaterialLibrary.CreateDynamicMaterialInstance` "/Game/Assets/Materials/M_Glow.M_Glow"))
  (bind _output_get (set `self.MatInstance` _returnvalue))
  (`PrimitiveComponent.SetMaterial` (`self.Mesh`) 0 _output_get)
  (`MaterialInstanceDynamic.SetScalarParameterValue` (`self.MatInstance`) "Glow" 0.0)
  (`AudioComponent.Play` (`self.EngineSound`) 0.0))

(event `self.ReceiveTick`
  (params (DeltaSeconds :type "Float (single-precision)"))
  (`|ExecutionSequence`
    (:`then_0`
      ;[1 1 1] Måns' stuff
      (bind _output_get (set `self.Health` (`KismetMathLibrary.FClamp` (- (`self.Health`) (* (`self.DegradationSpeed`) (`GameplayStatics.GetWorldDeltaSeconds`))) 0.0 100.0)))
      (`MaterialInstanceDynamic.SetScalarParameterValue` (`self.MatInstance`) "Glow" (/ _output_get 100.0)))
    (:`then_1`
      ;[1 1 1] Set Engine Sound
      (`AudioComponent.SetVolumeMultiplier` (`self.EngineSound`) (/ (`self.Health`) 100.0)))))

(fn `Repair`
  (params (Amount :type "Float (double-precision)"))
  (bind _output_get (set `self.Health` (`KismetMathLibrary.FClamp` (+ (`self.Health`) Amount) 0.0 100.0)))
  (`MaterialInstanceDynamic.SetScalarParameterValue` (`self.MatInstance`) "Glow" (/ _output_get 100.0)))

(fn `UserConstructionScript`)