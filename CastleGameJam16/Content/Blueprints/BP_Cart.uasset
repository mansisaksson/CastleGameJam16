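; BP_Cart creates cart movement by sliding the world actor (BP_Root) along negative Y, while the cart's own transform is left untouched.
; BeginPlay caches the BP_Root found in the level as WorldActor.
; Each Tick reads Health from the BP_Furnace child actor, maps the lost fraction through DegradationCurve and scales it by MaxSpeed.
; The resulting speed, multiplied by delta time, offsets WorldActor's location.
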(event `self.ReceiveBeginPlay`
  (bind _outactors (`GameplayStatics.GetAllActorsOfClass` "/Game/Blueprints/BP_Root.BP_Root_C"))
  (for _array_element _outactors
    (set `self.WorldActor` _array_element)))

(event `self.ReceiveTick`
  (params (DeltaSeconds :type "Float (single-precision)"))
  (bind (_returnvalue_x _returnvalue_y) (`KismetMathLibrary.BreakVector` (`self.K2_GetActorLocation` (`self.WorldActor`))))
  (`|ExecutionSequence`
    (:`then_0`
      ;[1 1 1] Calculate speed
      (bind _asbp_furnace (cast `/Game/Blueprints/BP_Furnace` (`ChildActorComponent.ChildActor` (`self.Furnace`))))
      (set `self.CurrentSpeed` (* (`CurveFloat.GetFloatValue` (`self.DegradationCurve`) (- 1.0 (/ (`/Game/Blueprints/BP_Furnace.Health` _asbp_furnace) 100.0))) (`self.MaxSpeed`))))
    (:`then_1`
      ;[1 1 1] Move The Cart
      (`self.K2_SetActorLocation` (`self.WorldActor`) (`KismetMathLibrary.MakeVector` 0.0 (- _returnvalue_y (* (`GameplayStatics.GetWorldDeltaSeconds`) (`self.CurrentSpeed`)))) false false))))

(fn `UserConstructionScript`)