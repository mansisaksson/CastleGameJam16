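; BP_TuutTuut is a VR pull-down handle, apparently for a horn, that the player grabs with the right motion controller trigger.
; Overlapping the mesh stores the player's component and enables custom depth as a highlight.
; While held, Tick follows that component's height within a short range below the start Z; otherwise it eases back up.
; The TUUT component is stopped on BeginPlay and never played here.
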(event `self.ReceiveBeginPlay`
  (bind (_returnvalue_x _returnvalue_y _returnvalue_z) (`KismetMathLibrary.BreakVector` (`self.K2_GetActorLocation`)))
  (set `self.StartZ` _returnvalue_z)
  (`AudioComponent.Stop` (`self.TUUUUUUUUUUUUUT`)))

(event `self.ReceiveTick`
  (params (DeltaSeconds :type "Float (single-precision)"))
  (bind (_returnvalue_x _returnvalue_y) (`KismetMathLibrary.BreakVector` (`self.K2_GetActorLocation`)))
  (bind (_returnvalue_x_2 _returnvalue_y_2) (`KismetMathLibrary.BreakVector` (`self.K2_GetActorLocation`)))
  (bind (_returnvalue_x_3 _returnvalue_y_3 _returnvalue_z) (`KismetMathLibrary.BreakVector` (`SceneComponent.K2_GetComponentLocation` (`self.OverlapCompRef`))))
  (if (`self.TuuTuutPressed`)
    ;[1 1 1] Follow player hand
    (`self.K2_SetActorLocation` (`KismetMathLibrary.MakeVector` _returnvalue_x_2 _returnvalue_y_2 (`KismetMathLibrary.FClamp` _returnvalue_z (- (`self.StartZ`) 30.0) (`self.StartZ`))))
    (else
      ;[1 1 1] Go Back To start pos
      (`self.K2_SetActorLocation` (`KismetMathLibrary.VLerp` (`self.K2_GetActorLocation`) (`KismetMathLibrary.MakeVector` _returnvalue_x _returnvalue_y (`self.StartZ`)) (* (`GameplayStatics.GetWorldDeltaSeconds`) 0.5))))))

(event `self.StaticMesh.OnComponentBeginOverlap`
  (params (OverlappedComponent :type "PrimitiveComponent Object Reference") (OtherActor :type "Actor Object Reference") (OtherComp :type "PrimitiveComponent Object Reference") (OtherBodyIndex :type Integer) (bFromSweep :type Boolean) (SweepResult :type "HitResult Structure (by ref)"))
  (cast `/Game/Blueprints/BP_Player` OtherActor)
  (set `self.OverlapCompRef` OtherComp)
  (`PrimitiveComponent.SetRenderCustomDepth` (`self.StaticMesh`) true)
  (set `self.PlayerIsOverlapping` true))

(event `self.StaticMesh.OnComponentEndOverlap`
  (params (OverlappedComponent :type "PrimitiveComponent Object Reference") (OtherActor :type "Actor Object Reference") (OtherComp :type "PrimitiveComponent Object Reference") (OtherBodyIndex :type Integer))
  (cast `/Game/Blueprints/BP_Player` OtherActor)
  (`PrimitiveComponent.SetRenderCustomDepth` (`self.StaticMesh`) false)
  (set `self.PlayerIsOverlapping` false)
  (set `self.TuuTuutPressed` false))

(event `Key|MotionController_Right_Trigger` :consume false
  (params (Key :type "Key Structure" :default "AnyKey"))
  (:`Pressed`
    (if (`self.PlayerIsOverlapping`)
      (set `self.TuuTuutPressed` true)))
  (:`Released`
    (set `self.TuuTuutPressed` false)))

(fn `UserConstructionScript`)