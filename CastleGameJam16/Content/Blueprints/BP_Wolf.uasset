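; Wolf enemy that stalks the player, pounces and restarts the level on a catch.
; Tick drives three states: drifting along Y at a random speed with a sine bob, homing on the player, and lunging to the camera.
; The attack starts with a growl after a delay that lengthens with the BP_Cart's speed ratio.
; Sphere overlap with the player triggers the kill lunge, then restarts the level after a short delay.
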(event `self.ReceiveBeginPlay`
  (bind _outactors (`GameplayStatics.GetAllActorsOfClass` "/Game/Blueprints/BP_Cart.BP_Cart_C"))
  (for _array_element _outactors
    (set `self.CartRef` _array_element)
    (set `self.DeltaSpeed` (`KismetMathLibrary.RandomFloatInRange` -250.0 250.0))))

(event `self.ReceiveTick`
  (params (DeltaSeconds :type "Float (single-precision)"))
  (bind (_returnvalue_x _returnvalue_y _returnvalue_z) (`KismetMathLibrary.BreakVector` (`self.K2_GetActorLocation`)))
  (bind _cartref (`self.CartRef`))
  (if (`self.IsKillingPlayer`)
    ;[1 1 1] Kill Player
    (bind _asbp_player (cast `/Game/Blueprints/BP_Player` (`GameplayStatics.GetPlayerPawn` 0)))
    (bind _camera (`/Game/Blueprints/BP_Player.Camera` _asbp_player))
    (bind _returnvalue (`SceneComponent.K2_GetComponentLocation` _camera))
    (`self.K2_SetActorLocation` (`KismetMathLibrary.VLerp` (`self.K2_GetActorLocation`) (+ _returnvalue (* (`SceneComponent.GetForwardVector` _camera) 50.0)) (* (`GameplayStatics.GetWorldDeltaSeconds`) 10.0)))
    (`self.K2_SetActorRotation` (`KismetMathLibrary.FindLookAtRotation` (`self.K2_GetActorLocation`) _returnvalue))
    (elif (`self.IsAttacking`)
      ;[1 1 1] Attack Player
      (`self.K2_SetActorLocation` (`KismetMathLibrary.VLerp` (`self.K2_GetActorLocation`) (+ (0.0 0.0 150.0) (`self.K2_GetActorLocation` (`GameplayStatics.GetPlayerPawn` 0))) (* (`GameplayStatics.GetWorldDeltaSeconds`) 1.0)))
      (`self.K2_SetActorRotation` (`KismetMathLibrary.FindLookAtRotation` (`self.K2_GetActorLocation`) (+ (0.0 0.0 150.0) (`self.K2_GetActorLocation` (`GameplayStatics.GetPlayerPawn` 0)))))
      (else
        (`|ExecutionSequence`
          (:`then_0`
            ;[1 1 1] Plan Attack
            (`KismetSystemLibrary.Delay` (+ 5.0 (* (/ (`/Game/Blueprints/BP_Cart.CurrentSpeed` _cartref) (`/Game/Blueprints/BP_Cart.MaxSpeed` _cartref)) 15.0)))
            (set `self.IsAttacking` true)
            (`GameplayStatics.PlaySoundAtLocation` "/Game/Audio/Growl.Growl" (`self.K2_GetActorLocation`)))
          (:`then_1`
            ;[1 1 1] Do Movement
            (`self.K2_SetActorLocation` (`KismetMathLibrary.MakeVector` _returnvalue_x (+ _returnvalue_y (* (`self.DeltaSpeed`) (`GameplayStatics.GetWorldDeltaSeconds`))) (+ _returnvalue_z (* (`KismetMathLibrary.Sin` (* (`KismetSystemLibrary.GetGameTimeInSeconds`) 8.0)) 1.0))))))))))

(event `self.Sphere.OnComponentBeginOverlap`
  (params (OverlappedComponent :type "PrimitiveComponent Object Reference") (OtherActor :type "Actor Object Reference") (OtherComp :type "PrimitiveComponent Object Reference") (OtherBodyIndex :type Integer) (bFromSweep :type Boolean) (SweepResult :type "HitResult Structure (by ref)"))
  (cast `/Game/Blueprints/BP_Player` OtherActor)
  (`GameplayStatics.PlaySoundAtLocation` "/Game/Audio/GrowlAttack.GrowlAttack" (`self.K2_GetActorLocation`))
  (set `self.IsKillingPlayer` true)
  (`KismetSystemLibrary.Delay` 2.0)
  (`KismetSystemLibrary.ExecuteConsoleCommand` "RestartLevel"))

(fn `UserConstructionScript`)