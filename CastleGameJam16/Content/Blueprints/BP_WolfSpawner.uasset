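; Spawner actor that, while active, releases wolves at random TargetPoints in the level, each with a howl.
; A Delay in Tick paces spawns, with a float curve over active time scaling the extra wait added to the base interval.
; Tick also prunes invalid wolves from its list and slowly eases the drum track's volume toward the living count, beside an ambience track started at BeginPlay.
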(event `self.ReceiveBeginPlay`
  (bind _outactors (`GameplayStatics.GetAllActorsOfClass` "/Script/Engine.TargetPoint"))
  (set `self.TargetPoints` _outactors)
  (`AudioComponent.Play` (`self.Drums`) 0.0)
  (`AudioComponent.SetVolumeMultiplier` (`self.Drums`) 0.0)
  (`AudioComponent.Play` (`self.Ambience`) 0.0))

(event `self.ReceiveTick`
  (params (DeltaSeconds :type "Float (single-precision)"))
  (bind _targetpoints (`self.TargetPoints`))
  (bind _drums (`self.Drums`))
  (bind _returnvalue_location (`KismetMathLibrary.BreakTransform` (`self.GetTransform` (`KismetArrayLibrary.Array_Get` _targetpoints (`KismetMathLibrary.RandomIntegerInRange` 0 (- (`KismetArrayLibrary.Array_Length` _targetpoints) 1))))))
  (`|ExecutionSequence`
    (:`then_0`
      ;[1 1 1] Spawn Wolves
      (if (`self.IsActive`)
        (set `self.TimeActive` (+ (`self.TimeActive`) (`GameplayStatics.GetWorldDeltaSeconds`)))
        (`KismetSystemLibrary.Delay` (+ (`self.BaseSpawnRate`) (* (- 1.0 (`CurveFloat.GetFloatValue` (`self.SpawnCurve`) (/ (`self.TimeActive`) (`self.MaxSpawnRateTime`)))) (`self.MaxAddedSpawnRate`))))
        (if (`self.IsActive`)
          (bind _returnvalue (`|SpawnActorFromClass` "/Game/Blueprints/BP_Wolf.BP_Wolf_C" (`KismetMathLibrary.MakeTransform` _returnvalue_location (struct :`Yaw` 90.0)) "AlwaysSpawn" "OverrideRootScale"))
          (`GameplayStatics.PlaySoundAtLocation` "/Game/Audio/SpawnHowl.SpawnHowl" (`self.K2_GetActorLocation` _returnvalue))
          (`KismetArrayLibrary.Array_Add` (`self.Wolves`) _returnvalue))))
    (:`then_1`
      ;[1 1 1] Play dem sweet Drums
      (for _array_element (`self.Wolves`)
        (`/Engine/EditorBlueprintResources/StandardMacros.IsValid` _array_element
          (:`Is Not Valid`
            (`KismetArrayLibrary.Array_RemoveItem` (`self.Wolves`) _array_element))))
      (`AudioComponent.SetVolumeMultiplier` _drums (`KismetMathLibrary.Lerp` (`AudioComponent.VolumeMultiplier` _drums) (`KismetMathLibrary.FClamp` (/ (`KismetMathLibrary.Conv_IntToDouble` (`KismetArrayLibrary.Array_Length` (`self.Wolves`))) 5.0)) (* (`GameplayStatics.GetWorldDeltaSeconds`) 0.1))))))

(fn `UserConstructionScript`)