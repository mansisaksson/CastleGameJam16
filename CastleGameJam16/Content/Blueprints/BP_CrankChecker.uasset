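; BP_CrankChecker detects full turns of a BP_Crank and spawns coal as the reward.
; Four box triggers each count overlaps from the crank, and once all four have been hit in any order, the counters reset and one turn is recorded.
; Every second recorded turn resets the tally and spawns a BP_Coal at the SpawnLocation transform.
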(event `self.Box1.OnComponentBeginOverlap`
  (params (OverlappedComponent :type "PrimitiveComponent Object Reference") (OtherActor :type "Actor Object Reference") (OtherComp :type "PrimitiveComponent Object Reference") (OtherBodyIndex :type Integer) (bFromSweep :type Boolean) (SweepResult :type "HitResult Structure (by ref)"))
  (cast `/Game/Blueprints/BP_Crank` OtherActor)
  (set `self.BoxV1` (+ (`self.BoxV1`) 1))
  (if (and (> (`self.BoxV1`) 0) (> (`self.BoxV2`) 0) (> (`self.BoxV3`) 0) (> (`self.BoxV4`) 0)) :!label _label
    (set `self.BoxV1` 0)
    (set `self.BoxV2` 0)
    (set `self.BoxV3` 0)
    (set `self.BoxV4` 0)
    (bind _output_get (set `self.Cranks` (+ (`self.Cranks`) 1)))
    (if (>= _output_get 2)
      (set `self.Cranks` 0)
      (`|SpawnActorFromClass` "/Game/Blueprints/BP_Coal.BP_Coal_C" (`SceneComponent.K2_GetComponentToWorld` (`self.Spawn Location`)) "AlwaysSpawn" "OverrideRootScale"))))

(event `self.Box2.OnComponentBeginOverlap`
  (params (OverlappedComponent :type "PrimitiveComponent Object Reference") (OtherActor :type "Actor Object Reference") (OtherComp :type "PrimitiveComponent Object Reference") (OtherBodyIndex :type Integer) (bFromSweep :type Boolean) (SweepResult :type "HitResult Structure (by ref)"))
  (cast `/Game/Blueprints/BP_Crank` OtherActor)
  (set `self.BoxV2` (+ (`self.BoxV2`) 1))
  (goto _label))

(event `self.Box3.OnComponentBeginOverlap`
  (params (OverlappedComponent :type "PrimitiveComponent Object Reference") (OtherActor :type "Actor Object Reference") (OtherComp :type "PrimitiveComponent Object Reference") (OtherBodyIndex :type Integer) (bFromSweep :type Boolean) (SweepResult :type "HitResult Structure (by ref)"))
  (cast `/Game/Blueprints/BP_Crank` OtherActor)
  (set `self.BoxV3` (+ (`self.BoxV3`) 1))
  (goto _label))

(event `self.Box4.OnComponentBeginOverlap`
  (params (OverlappedComponent :type "PrimitiveComponent Object Reference") (OtherActor :type "Actor Object Reference") (OtherComp :type "PrimitiveComponent Object Reference") (OtherBodyIndex :type Integer) (bFromSweep :type Boolean) (SweepResult :type "HitResult Structure (by ref)"))
  (cast `/Game/Blueprints/BP_Crank` OtherActor)
  (set `self.BoxV4` (+ (`self.BoxV4`) 1))
  (goto _label))

(fn `UserConstructionScript`)