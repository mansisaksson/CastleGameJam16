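; BP_Bucket is a tar bucket that restores a BP_Torch when the torch overlaps it.
; A torch below or otherwise not at full health is extinguished and reset to full, and each use drains a clamped amount of BucketHealth.
; The remaining health is converted into a frame time on ABP_Bucket, so the Tar mesh's animation shows the level dropping.
; Nothing stops refills once the bucket is empty.
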(event `self.ReceiveTick`
  (params (DeltaSeconds :type "Float (single-precision)")))

(event `self.Bucket.OnComponentBeginOverlap`
  (params (OverlappedComponent :type "PrimitiveComponent Object Reference") (OtherActor :type "Actor Object Reference") (OtherComp :type "PrimitiveComponent Object Reference") (OtherBodyIndex :type Integer) (bFromSweep :type Boolean) (SweepResult :type "HitResult Structure (by ref)"))
  (bind _asbp_torch (cast `/Game/Blueprints/BP_Torch` OtherActor))
  (if (not (== (`/Game/Blueprints/BP_Torch.Health` _asbp_torch) 100.0))
    (`/Game/Blueprints/BP_Torch.Extinguish` _asbp_torch)
    (set `/Game/Blueprints/BP_Torch.Health` 100.0 _asbp_torch)
    (set `self.BucketHealth` (`KismetMathLibrary.FClamp` (- (`self.BucketHealth`) 10.0) 0.0 100.0))
    ;[1 1 1] Set Tar Height
    (bind _asabp_bucket (cast `/Game/Assets/Bucket/ABP_Bucket` (`SkeletalMeshComponent.GetAnimInstance` (`self.Tar`))))
    (set `/Game/Assets/Bucket/ABP_Bucket.FrameTime` (* (- 1.0 (/ (`self.BucketHealth`) 100.0)) 4.16666667) _asabp_bucket)))

(fn `UserConstructionScript`)