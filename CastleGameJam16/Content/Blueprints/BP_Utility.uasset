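; BP_Utility is a physics prop actor that can be highlighted, picked up and released.
; SetHighLight toggles custom depth rendering on UtilityMesh, as used for outline effects.
; PickUp turns off the mesh's physics and collision, and Release detaches it in world space and restores both.
; The event graph is empty and PickUp does no attaching, so these functions only act when called.
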(fn `PickUp`
  (bind _utilitymesh (`self.UtilityMesh`))
  (`PrimitiveComponent.SetSimulatePhysics` _utilitymesh false)
  (`PrimitiveComponent.SetCollisionEnabled` _utilitymesh "NoCollision"))

(fn `Release`
  (bind _utilitymesh (`self.UtilityMesh`))
  (`SceneComponent.K2_DetachFromComponent` _utilitymesh "KeepWorld" "KeepWorld" "KeepWorld" true)
  (`PrimitiveComponent.SetSimulatePhysics` _utilitymesh true)
  (`PrimitiveComponent.SetCollisionEnabled` _utilitymesh "QueryAndPhysics"))

(fn `SetHighLight`
  (params (Highlight :type Boolean))
  (`PrimitiveComponent.SetRenderCustomDepth` (`self.UtilityMesh`) Highlight))

(fn `UserConstructionScript`)