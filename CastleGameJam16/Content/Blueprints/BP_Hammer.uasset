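; BP_Hammer is a hammer tool that repairs a BP_Furnace when swung into it.
; An overlap on its UtilityMesh applies a fixed repair if HandVelocity exceeds a small threshold, with a brief CanHit cooldown preventing rapid repeat hits.
; Any physical hit on the mesh plays a floor thud sound at the actor's location, and Tick only calls the parent.
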(event `self.ReceiveBeginPlay`)

(event `self.ReceiveTick`
  (params (DeltaSeconds :type "Float (single-precision)"))
  (`parent.ReceiveTick` DeltaSeconds))

(event `self.UtilityMesh.OnComponentBeginOverlap`
  (params (OverlappedComponent :type "PrimitiveComponent Object Reference") (OtherActor :type "Actor Object Reference") (OtherComp :type "PrimitiveComponent Object Reference") (OtherBodyIndex :type Integer) (bFromSweep :type Boolean) (SweepResult :type "HitResult Structure (by ref)"))
  (bind _asbp_furnace (cast `/Game/Blueprints/BP_Furnace` OtherActor))
  (if (and (`self.CanHit`) (> (`self.HandVelocity`) 0.1))
    (`/Game/Blueprints/BP_Furnace.Repair` _asbp_furnace 30.0)
    (set `self.CanHit` false)
    (`KismetSystemLibrary.Delay` 0.1)
    (set `self.CanHit` true)))

(event `self.UtilityMesh.OnComponentHit`
  (params (HitComponent :type "PrimitiveComponent Object Reference") (OtherActor :type "Actor Object Reference") (OtherComp :type "PrimitiveComponent Object Reference") (NormalImpulse :type "Vector Structure") (Hit :type "HitResult Structure (by ref)"))
  ;[1 1 1] Hit Floor Thud
  (`GameplayStatics.PlaySoundAtLocation` "/Game/Audio/HitFloor.HitFloor" (`self.K2_GetActorLocation`)))

(fn `UserConstructionScript`)