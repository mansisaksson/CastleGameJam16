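; Pickup torch that lights on contact with a furnace, burns down over time and kills wolves when swung.
; While burning, Tick drains Health, which drives glow and light intensity, hides particles when low and extinguishes the torch at zero.
; While lit and held, a sphere collider sits beyond the torch along the camera-to-torch direction, tracking overlapping wolves.
; Sufficient HandVelocity triggers destruction of those tracked wolves.
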(event `self.ReceiveBeginPlay`
  (set `self.MaxIntensity` (`LightComponentBase.Intensity` (`self.PointLight`)))
  (bind _returnvalue (`KismetMaterialLibrary.CreateDynamicMaterialInstance` "/Game/Assets/Materials/M_TorchHead.M_TorchHead"))
  (bind _output_get (set `self.MatInstance` _returnvalue))
  (`PrimitiveComponent.SetMaterial` (`self.UtilityMesh`) 0 _output_get)
  (`PrimitiveComponent.SetCollisionEnabled` (`self.Sphere`) "NoCollision"))

(event `self.ReceiveTick`
  (params (DeltaSeconds :type "Float (single-precision)"))
  (bind _wolvesthatmaydie (`self.WolvesThatMayDie`))
  (bind _sphere (`self.Sphere`))
  (bind _particlesystem (`self.ParticleSystem`))
  (`parent.ReceiveTick` DeltaSeconds)
  (`|ExecutionSequence`
    (:`then_0`
      ;[1 1 1] HP loss
      (if (`self.IsBurning`)
        (bind _output_get (set `self.Health` (`KismetMathLibrary.FClamp` (- (`self.Health`) (* (`GameplayStatics.GetWorldDeltaSeconds`) 1.0)) 0.0 100.0)))
        (bind _returnvalue (/ _output_get 100.0))
        (`MaterialInstanceDynamic.SetScalarParameterValue` (`self.MatInstance`) "GlowStrength" _returnvalue)
        (`LightComponent.SetIntensity` (`self.PointLight`) (* _returnvalue (`self.MaxIntensity`)))
        (if (== _output_get 0.0)
          (`self.Extinguish`)
          (elif (< _output_get 20.0)
            (`SceneComponent.SetVisibility` _particlesystem false false)
            (else
              (`SceneComponent.SetVisibility` _particlesystem true false))))))
    (:`then_1`
      ;[1 1 1] Update Collider
      (if (and (`self.IsBurning`) (`self.IsPickedUp`))
        (`PrimitiveComponent.SetCollisionEnabled` _sphere "QueryOnly")
        (bind _asbp_player (cast `/Game/Blueprints/BP_Player` (`GameplayStatics.GetPlayerPawn` 0)))
        (`SceneComponent.K2_SetWorldLocation` (`self.Sphere`) (+ (`self.K2_GetActorLocation`) (* (`KismetMathLibrary.Normal` (- (`self.K2_GetActorLocation`) (`SceneComponent.K2_GetComponentLocation` (`/Game/Blueprints/BP_Player.Camera` _asbp_player)))) (`SphereComponent.SphereRadius` (`self.Sphere`)))) true false)
        (if (> (`self.HandVelocity`) 0.1)
          (for _array_element _wolvesthatmaydie
            (`self.K2_DestroyActor` _array_element)
            (`KismetArrayLibrary.Array_Clear` _wolvesthatmaydie)))
        (else
          (`PrimitiveComponent.SetCollisionEnabled` _sphere "NoCollision"))))))

(event `self.UtilityMesh.OnComponentBeginOverlap`
  (params (OverlappedComponent :type "PrimitiveComponent Object Reference") (OtherActor :type "Actor Object Reference") (OtherComp :type "PrimitiveComponent Object Reference") (OtherBodyIndex :type Integer) (bFromSweep :type Boolean) (SweepResult :type "HitResult Structure (by ref)"))
  (cast `/Game/Blueprints/BP_Furnace` OtherActor)
  (`self.Ignite`))

(event `self.UtilityMesh.OnComponentHit`
  (params (HitComponent :type "PrimitiveComponent Object Reference") (OtherActor :type "Actor Object Reference") (OtherComp :type "PrimitiveComponent Object Reference") (NormalImpulse :type "Vector Structure") (Hit :type "HitResult Structure (by ref)"))
  ;[1 1 1] Hit Floor Thud
  (`GameplayStatics.PlaySoundAtLocation` "/Game/Audio/HitFloor.HitFloor" (`self.K2_GetActorLocation`)))

(event `self.Sphere.OnComponentBeginOverlap`
  (params (OverlappedComponent :type "PrimitiveComponent Object Reference") (OtherActor :type "Actor Object Reference") (OtherComp :type "PrimitiveComponent Object Reference") (OtherBodyIndex :type Integer) (bFromSweep :type Boolean) (SweepResult :type "HitResult Structure (by ref)"))
  (bind _asbp_wolf (cast `/Game/Blueprints/BP_Wolf` OtherActor))
  (`KismetArrayLibrary.Array_Add` (`self.WolvesThatMayDie`) _asbp_wolf))

(event `self.Sphere.OnComponentEndOverlap`
  (params (OverlappedComponent :type "PrimitiveComponent Object Reference") (OtherActor :type "Actor Object Reference") (OtherComp :type "PrimitiveComponent Object Reference") (OtherBodyIndex :type Integer))
  (bind _asbp_wolf (cast `/Game/Blueprints/BP_Wolf` OtherActor))
  (`KismetArrayLibrary.Array_RemoveItem` (`self.WolvesThatMayDie`) _asbp_wolf))

(fn `Extinguish`
  (if (`self.IsBurning`)
    (`GameplayStatics.PlaySoundAtLocation` "/Game/Audio/LightTurnOff.LightTurnOff" (`self.K2_GetActorLocation`))
    (`AudioComponent.Stop` (`self.TorchSound`)))
  (set `self.IsBurning` false)
  (`SceneComponent.SetVisibility` (`self.ParticleSystem`) false false)
  (`SceneComponent.SetVisibility` (`self.PointLight`) false false)
  (`MaterialInstanceDynamic.SetScalarParameterValue` (`self.MatInstance`) "GlowStrength" 0.0))

(fn `Ignite`
  (bind _output_get (set `self.IsBurning` (> (`self.Health`) 0.0)))
  (if _output_get
    (`SceneComponent.SetVisibility` (`self.ParticleSystem`) true false)
    (`SceneComponent.SetVisibility` (`self.PointLight`) true false)
    (`GameplayStatics.PlaySoundAtLocation` "/Game/Audio/LightTurnOn.LightTurnOn" (`self.K2_GetActorLocation`))
    (`AudioComponent.Play` (`self.TorchSound`) 0.0)))

(fn `UserConstructionScript`
  (`parent.UserConstructionScript`))